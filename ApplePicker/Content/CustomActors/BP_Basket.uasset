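; BP_Basket is the player-controlled basket for an apple-catching game, sliding horizontally along the bottom of the play area.
; Each tick it deprojects the mouse position to world space and teleports to that clamped Y, with X at zero and Z at BottomY.
; Overlapping an actor tagged Apple notifies BP_ApplePickerGameMode through AppleCaught, then destroys that actor.
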(event Collision|EventActorBeginOverlap
  (params (OtherActor :type Actor%20Object%20Reference))
  (if (Actor|ActorHasTag OtherActor "Apple")
    (bind _asbp_apple_picker_game_mode (Utilities|Casting|CastToBP_ApplePickerGameMode (Game|GetGameMode)))
    (Default|AppleCaught _asbp_apple_picker_game_mode)
    (Actor|DestroyActor OtherActor)))

(event EventTick
  (params (DeltaSeconds :type Float%20%28single-precision%29))
  (Class|WidgetLayoutLibrary|GetMousePositiononViewport)
  (Transformation|SetActorLocation (Math|Vector|MakeVector 0.0 (Math|Float|Clamp(Float) (.Y (Math|Vector|BreakVector (.WorldLocation (Game|Player|ConvertMouseLocationToWorldSpace (Game|GetPlayerController 0))))) -7e+02 7e+02) (Variables|Default|GetbottomY)) false true))

(fn ConstructionScript)