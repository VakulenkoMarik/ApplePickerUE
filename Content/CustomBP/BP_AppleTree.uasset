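; BP_AppleTree is an actor that moves side to side and drops apples, as in an apple-catching game.
; A looping timer started on BeginPlay spawns a BP_Apple at the tree's location.
; Tick offsets the tree along local Y by Speed, with what appears to be a direction flip at the left and right edges or on a random per-frame roll, making the turn rate frame-rate dependent.
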(event Custom|DropApple
  (Game|SpawnActorfromClass "/Game/CustomBP/BP_Apple.BP_Apple_C" (Math|Conversions|ToTransform(Vector) (Transformation|GetActorLocation)) "AlwaysSpawn" 0 0))

(event EventTick
  (params (DeltaSeconds :type Float%20%28single-precision%29))
  (bind _returnvalue (Transformation|GetActorLocation))
  (bind _y (Math|Vector|BreakVector _returnvalue))
  (Transformation|AddActorLocalOffset (Math|Vector|MakeVector 0.0 (* DeltaSeconds (Variables|Default|Getspeed)) 0.0) false false)
  (if (or (or (>= _y (Variables|Default|GetrightEdge)) (<= _y (Variables|Default|GetleftEdge))) (== (Math|Random|RandomIntegerinRange 0 (Variables|Default|GetchanceToChangeDir)) (Variables|Default|GetchanceToChangeDir)))
    (Math|Float|NegateFloat (Variables|Default|Getspeed))))

(event EventBeginPlay
  (Utilities|Time|SetTimerbyFunctionName 0 "DropApple" 1.0 true 1.5))

(fn ConstructionScript)